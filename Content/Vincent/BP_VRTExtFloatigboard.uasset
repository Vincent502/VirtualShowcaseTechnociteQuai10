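; BP_VRTExtFloatigboard is a floating board actor whose Widget follows the player camera's orientation while IsFollowing is set.
; Each Tick interpolates from the actor's transform toward a camera-derived target and applies the result to the Widget in world space.
; The location target is only the camera forward vector's X scaled, without camera position; the rotation target is the camera rotation.
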(event `self.ReceiveTick`
  (params (DeltaSeconds :type "Float (single-precision)"))
  (bind _returnvalue (`GameplayStatics.GetPlayerCameraManager` 0))
  (bind _returnvalue_2 (`GameplayStatics.GetWorldDeltaSeconds`))
  (if (`self.IsFollowing`)
    (bind _output_get (set `self.TargetLocation` (* (`self.GetActorForwardVector` _returnvalue) (100.0 0.0 0.0))))
    (`SceneComponent.K2_SetWorldLocationAndRotation` (`self.Widget`) (`KismetMathLibrary.VInterpTo` (`self.K2_GetActorLocation`) _output_get _returnvalue_2 5.0) (`KismetMathLibrary.RInterpTo` (`self.K2_GetActorRotation`) (`PlayerCameraManager.GetCameraRotation` _returnvalue) _returnvalue_2 5.0) false false)))

(fn `UserConstructionScript`)