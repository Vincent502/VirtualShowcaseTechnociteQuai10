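; BP_Interface is an actor that carries an interactable UI widget (IsdkInteractableWidget) and keeps it facing the player.
; Every tick it places the widget slightly above the scene root and rotates it toward the player camera with a look-at rotation.
; BeginPlay casts the hosted user widget to NewWidgetBlueprint but does nothing with the result.
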(event `self.ReceiveBeginPlay`
  (cast `/Game/Vincent/NewWidgetBlueprint` (`WidgetComponent.GetUserWidgetObject` (`IsdkInteractableWidgetComponent.Widget` (`self.IsdkInteractableWidget`)))))

(event `self.ReceiveTick`
  (params (DeltaSeconds :type "Float (single-precision)"))
  (bind _isdkinteractablewidget (`self.IsdkInteractableWidget`))
  (`SceneComponent.K2_SetWorldLocationAndRotation` _isdkinteractablewidget (+ (`SceneComponent.K2_GetComponentLocation` (`self.DefaultSceneRoot`)) (0.0 0.0 10.0)) (`KismetMathLibrary.FindLookAtRotation` (`SceneComponent.K2_GetComponentLocation` _isdkinteractablewidget) (`PlayerCameraManager.GetCameraLocation` (`GameplayStatics.GetPlayerCameraManager` 0))) false false))

(fn `UserConstructionScript`)