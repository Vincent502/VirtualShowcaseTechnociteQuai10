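; BP_TextFlottant is a floating text actor whose widget component displays a UI_TextFloatingboard and drifts after the player camera.
; Each tick, FloatingText interpolates from the widget's world transform toward the camera's location and yaw, then applies the result to the actor for a lagged follow.
; BeginPlay caches the widget reference, but the check on its visibility toggle is disconnected, so the follow always runs.
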(event `self.ReceiveBeginPlay`
  (bind _asui_text_floatingboard (cast `/Game/Vincent/UI_TextFloatingboard` (`WidgetComponent.GetWidget` (`self.Widget`))))
  (set `self.As UI Text Floatingboard` _asui_text_floatingboard))

(event `self.ReceiveTick`
  (params (DeltaSeconds :type "Float (single-precision)"))
  (`self.FloatingText` DeltaSeconds))

(fn `FloatingText`
  (params (DeltaTime :type "Float (double-precision)"))
  (bind _returnvalue (`GameplayStatics.GetPlayerCameraManager` 0))
  (bind _widget (`self.Widget`))
  (bind (_returnvalue_roll _returnvalue_pitch _returnvalue_yaw) (`KismetMathLibrary.BreakRotator` (`KismetMathLibrary.RInterpTo` (`SceneComponent.K2_GetComponentRotation` _widget) (`SceneComponent.K2_GetComponentRotation` (`Actor.RootComponent` _returnvalue)) DeltaTime 0.8)))
  (`self.K2_SetActorTransform` (`KismetMathLibrary.MakeTransform` (`KismetMathLibrary.VInterpTo` (`SceneComponent.K2_GetComponentLocation` _widget) (`SceneComponent.K2_GetComponentLocation` (`Actor.RootComponent` _returnvalue)) DeltaTime 0.6) (`KismetMathLibrary.MakeRotator` 0.0 0.0 _returnvalue_yaw))))

(fn `UserConstructionScript`)