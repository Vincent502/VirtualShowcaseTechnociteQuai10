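; BP_PositionDetection is a trigger actor that sends a target location to the BP_Guide_IA guide when its box is overlapped.
; On BeginPlay it moves its Sphere to the Pose location and caches the guide found in the level.
; Overlaps, except by the "Distance Grab Collider", call Deplacement, which passes a one-shot VInterpTo from guide to Sphere location into the guide's MaSuperCustome.
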(event `self.ReceiveBeginPlay`
  (`SceneComponent.K2_SetWorldLocation` (`self.Sphere`) (`self.Pose`) false false)
  (bind _returnvalue (`GameplayStatics.GetActorOfClass` "/Game/Sebastien/Blueprint/BP_Guide_IA.BP_Guide_IA_C"))
  (set `self.As BP Guide IA` _returnvalue))

(event `self.Box.OnComponentBeginOverlap`
  (params (OverlappedComponent :type "PrimitiveComponent Object Reference") (OtherActor :type "Actor Object Reference") (OtherComp :type "PrimitiveComponent Object Reference") (OtherBodyIndex :type Integer) (bFromSweep :type Boolean) (SweepResult :type "HitResult Structure (by ref)"))
  (if (not (`KismetStringLibrary.EqualEqual_StrStr` (`KismetSystemLibrary.GetObjectName` OtherComp) "Distance Grab Collider"))
    (`self.Deplacement`)))

(event `Deplacement`
  (bind _as_bp_guide_ia (`self.As BP Guide IA`))
  (`/Game/Sebastien/Blueprint/BP_Guide_IA.MaSuperCustome` _as_bp_guide_ia (`KismetMathLibrary.VInterpTo` (`self.K2_GetActorLocation` _as_bp_guide_ia) (`SceneComponent.K2_GetComponentLocation` (`self.Sphere`)))))

(fn `UserConstructionScript`)