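; BP_Classe is a trigger actor that sends the BP_Guide_IA guide to its location when something overlaps its box.
; At BeginPlay it finds the guide in the level and stores it as a Pawn.
; Any box overlap, with no filter on the overlapping actor, issues an AIMoveTo toward a VInterpTo result between the guide's location and the static mesh's world location.
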(event `self.ReceiveBeginPlay`
  (bind _returnvalue (`GameplayStatics.GetActorOfClass` "/Game/Sebastien/Blueprint/BP_Guide_IA.BP_Guide_IA_C"))
  (bind _output_get (set `self.IAGuide` _returnvalue))
  (bind _aspawn (cast `Pawn` _output_get))
  (set `self.Guide` _aspawn))

(event `self.Box.OnComponentBeginOverlap`
  (params (OverlappedComponent :type "PrimitiveComponent Object Reference") (OtherActor :type "Actor Object Reference") (OtherComp :type "PrimitiveComponent Object Reference") (OtherBodyIndex :type Integer) (bFromSweep :type Boolean) (SweepResult :type "HitResult Structure (by ref)"))
  (bind _guide (`self.Guide`))
  (`|AIMoveTo` _guide (`KismetMathLibrary.VInterpTo` (`self.K2_GetActorLocation` _guide) (`SceneComponent.K2_GetComponentLocation` (`self.StaticMeshComponent`))) null 6.0))

(event `self.ReceiveTick`
  (params (DeltaSeconds :type "Float (single-precision)")))

(fn `UserConstructionScript`)