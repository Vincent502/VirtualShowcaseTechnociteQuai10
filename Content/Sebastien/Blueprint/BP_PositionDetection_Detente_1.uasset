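; Trigger actor for the first "Detente" position, which signals the exit actor and moves the AI guide.
; At BeginPlay it caches the BP_PositionExit actor and places Sphere1 at Pose1 as the guide's target marker.
; A Box overlap, ignoring the Distance Grab Collider, activates two Detente functions on the exit.
; After a delay, it passes the guide a single interpolated location toward Sphere1.
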(event `self.ReceiveBeginPlay`
  (`parent.ReceiveBeginPlay`)
  (bind _returnvalue (`GameplayStatics.GetActorOfClass` "/Game/Sebastien/Blueprint/BP_PositionExit.BP_PositionExit_C"))
  (set `self.Exit` _returnvalue)
  (`SceneComponent.K2_SetWorldLocation` (`self.Sphere1`) (`self.Pose1`) false false))

(event `self.Box.OnComponentBeginOverlap`
  (params (OverlappedComponent :type "PrimitiveComponent Object Reference") (OtherActor :type "Actor Object Reference") (OtherComp :type "PrimitiveComponent Object Reference") (OtherBodyIndex :type Integer) (bFromSweep :type Boolean) (SweepResult :type "HitResult Structure (by ref)"))
  (bind _as_bp_guide_ia (`self.As BP Guide IA`))
  (bind _exit (`self.Exit`))
  (if (not (`KismetStringLibrary.EqualEqual_StrStr` (`KismetSystemLibrary.GetObjectName` OtherComp) "Distance Grab Collider"))
    (`/Game/Sebastien/Blueprint/BP_PositionExit.ActiveDetente` _exit)
    (`/Game/Sebastien/Blueprint/BP_PositionExit.ActiveDetene1` _exit)
    (`KismetSystemLibrary.Delay` 10.0)
    (`/Game/Sebastien/Blueprint/BP_Guide_IA.MaSuperCustome` _as_bp_guide_ia (`KismetMathLibrary.VInterpTo` (`self.K2_GetActorLocation` _as_bp_guide_ia) (`SceneComponent.K2_GetComponentLocation` (`self.Sphere1`))))))

(fn `UserConstructionScript`
  (`parent.UserConstructionScript`))