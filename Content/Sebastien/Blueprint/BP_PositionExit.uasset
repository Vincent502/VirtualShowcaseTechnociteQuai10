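; BP_PositionExit is an exit trigger that signals the BP_Guide_IA guide once five areas (kitchen, desk room, room, two zen zones) are flagged as visited.
; BeginPlay places its Sphere at the Pose location, finds the guide and clears the flags, which separate custom events set.
; Box overlaps, ignoring the guide and Distance Grab Colliders, then pass a VInterpTo from guide toward Sphere into the guide's MaSuperCustome.
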(event `self.ReceiveBeginPlay`
  (`SceneComponent.K2_SetWorldLocation` (`self.Sphere`) (`self.Pose`) false false)
  (bind _returnvalue (`GameplayStatics.GetActorOfClass` "/Game/Sebastien/Blueprint/BP_Guide_IA.BP_Guide_IA_C"))
  (set `self.As BP Guide IA` _returnvalue)
  (set `self.CountCollision` 0)
  (set `self.IsPassedKItchen` false)
  (set `self.IsPassedDeskRoom` false)
  (set `self.IsPassedRoom` false)
  (set `self.IsPassedZenZone1` false)
  (set `self.IsPassedZenZone` false))

(event `self.Box.OnComponentBeginOverlap`
  (params (OverlappedComponent :type "PrimitiveComponent Object Reference") (OtherActor :type "Actor Object Reference") (OtherComp :type "PrimitiveComponent Object Reference") (OtherBodyIndex :type Integer) (bFromSweep :type Boolean) (SweepResult :type "HitResult Structure (by ref)"))
  (bind _as_bp_guide_ia (`self.As BP Guide IA`))
  (if (`KismetStringLibrary.EqualEqual_StrStr` (`KismetSystemLibrary.GetObjectName` OtherComp) "Distance Grab Collider")
    _
    (elif (and (`self.IsPassedZenZone`) (`self.IsPassedZenZone1`) (`self.IsPassedKItchen`) (`self.IsPassedDeskRoom`) (`self.IsPassedRoom`))
      (if (not (== OtherActor (`self.As BP Guide IA`)))
        (`/Game/Sebastien/Blueprint/BP_Guide_IA.MaSuperCustome` _as_bp_guide_ia (`KismetMathLibrary.VInterpTo` (`self.K2_GetActorLocation` _as_bp_guide_ia) (`SceneComponent.K2_GetComponentLocation` (`self.Sphere`))))))))

(event `ActiveDetente`
  (set `self.IsPassedZenZone` true))

(event `ActiveDetene1`
  (set `self.IsPassedZenZone1` true))

(event `ActiveCuisine`
  (set `self.IsPassedKItchen` true))

(event `ActiveClasse`
  (set `self.IsPassedRoom` true))

(event `ActiveBureau`
  (set `self.IsPassedDeskRoom` true))

(fn `UserConstructionScript`)