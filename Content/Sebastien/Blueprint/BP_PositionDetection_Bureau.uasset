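; BP_PositionDetection_Bureau is a trigger actor that notifies the BP_PositionExit actor when something enters its Box, activating its "Bureau" state.
; On BeginPlay it finds and caches the BP_PositionExit instance with GetActorOfClass.
; On Box begin overlap it calls ActiveBureau on that exit, ignoring any component named "Distance Grab Collider" so the grab collider does not trigger it.
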(event `self.ReceiveBeginPlay`
  (`parent.ReceiveBeginPlay`)
  (bind _returnvalue (`GameplayStatics.GetActorOfClass` "/Game/Sebastien/Blueprint/BP_PositionExit.BP_PositionExit_C"))
  (set `self.Exit` _returnvalue))

(event `self.Box.OnComponentBeginOverlap`
  (params (OverlappedComponent :type "PrimitiveComponent Object Reference") (OtherActor :type "Actor Object Reference") (OtherComp :type "PrimitiveComponent Object Reference") (OtherBodyIndex :type Integer) (bFromSweep :type Boolean) (SweepResult :type "HitResult Structure (by ref)"))
  (if (not (`KismetStringLibrary.EqualEqual_StrStr` (`KismetSystemLibrary.GetObjectName` OtherComp) "Distance Grab Collider"))
    (`/Game/Sebastien/Blueprint/BP_PositionExit.ActiveBureau` (`self.Exit`))))

(fn `UserConstructionScript`
  (`parent.UserConstructionScript`))