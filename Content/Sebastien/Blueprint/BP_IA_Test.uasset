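; Test AI pawn that patrols the level's TargetPoint actors in a loop.
; BeginPlay gathers the points, then Chemin moves to the one at CurrentIndex, waits after arrival, increments with a hardcoded wrap at six and calls itself again.
; A random reachable-point wander event exists but is not started by BeginPlay.
; Player-following and distance-based wait-for-player guide logic are left disconnected, and the OnSeePawn handler is empty.
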(event `Chemin`
  (`KismetSystemLibrary.PrintText` (`KismetTextLibrary.Conv_IntToText` (`self.CurrentIndex`)))
  ;[0.6406 0.5778 0.02669 0.5] Deplacement Par point
  (for (_array_element _array_index) (`self.PointControl`)
    (if (== _array_index (`self.CurrentIndex`))
      (`|AIMoveTo` self (`self.K2_GetActorLocation` _array_element) null 10.0
        (:`OnSuccess`
          (`KismetSystemLibrary.Delay` 60.0)
          (bind _output_get (set `self.CurrentIndex` (+ 1 (`self.CurrentIndex`))))
          (if (== _output_get 6)
            (set `self.CurrentIndex` 0))
          (`KismetSystemLibrary.PrintString` (`KismetStringLibrary.Conv_IntToString` _output_get))
          (`self.Chemin`))))))

(event `Deplacement_IA`
  ;[0.599 0.5478 0.00312 0.5] Deplacement Aleatoire
  (`|AIMoveTo` self (`NavigationSystemV1.K2_GetRandomReachablePointInRadius` (`self.K2_GetActorLocation`) 3000.0 null null) null 100.0
    (:`OnSuccess`
      (`KismetSystemLibrary.Delay` 5.0)
      (`self.Deplacement_IA`))))

(event `self.ReceiveBeginPlay`
  (bind _returnvalue (`GameplayStatics.GetPlayerPawn` 0))
  (set `self.Player` _returnvalue)
  (set `self.PlayerRef` _returnvalue)
  (set `self.CurrentIndex` 0)
  (bind _outactors (`GameplayStatics.GetAllActorsOfClass` "/Script/Engine.TargetPoint"))
  (bind _output_get (set `self.PointControl` _outactors))
  (if (`KismetArrayLibrary.Array_IsNotEmpty` _output_get)
    (`self.Chemin`)))

(event `self.PawnSensing.OnSeePawn`
  (params (Pawn :type "Pawn Object Reference")))

(event `self.ReceiveTick`
  (params (DeltaSeconds :type "Float (single-precision)")))

(fn `UserConstructionScript`)